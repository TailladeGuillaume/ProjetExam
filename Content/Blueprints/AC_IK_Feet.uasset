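; Foot IK component that computes smoothed foot and pelvis offsets for a character on uneven ground.
; Each tick it line-traces beneath both foot bones from actor height, deriving height offsets and floor normals.
; The pelvis follows the larger offset, and all values are interpolated.
; Foot rotations use the floor-normal angle, but their axis crosses the up vector with a zero vector, yielding no valid tilt axis.
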(event `self.ReceiveTick`
  (params (DeltaSeconds :type "Float (single-precision)"))
  (set `self.DeltaSeconds` DeltaSeconds)
  ;[0 0.6863 1] Calcul Offset Pied Gauche
  (bind (_returnvalue _impactnormal) (`self.TraceFromRoot` (`self.LeftFootName`) (`self.TraceDistBelowCapsule`)))
  (set `self.LeftFootFloorNormal` _impactnormal)
  (set `self.LeftFootOffset` (`KismetMathLibrary.FInterpTo` (`self.LeftFootOffset`) _returnvalue (`self.DeltaSeconds`) (`self.InterpSpeed`)))
  ;[0 0.6863 1] Calcul offset Pied droit
  (bind (_returnvalue_2 _impactnormal_2) (`self.TraceFromRoot` (`self.RightFootName`) (`self.TraceDistBelowCapsule`)))
  (set `self.RightFootFloorNormal` _impactnormal_2)
  (set `self.RightFootOffset` (`KismetMathLibrary.FInterpTo` (`self.RightFootOffset`) _returnvalue_2 (`self.DeltaSeconds`) (`self.InterpSpeed`)))
  ;[0 0.6863 1] Calcul Offset Pelvis
  (set `self.PelvisOffset` (`KismetMathLibrary.FInterpTo` (`self.PelvisOffset`) (`KismetMathLibrary.FMax` (`self.LeftFootOffset`) (`self.RightFootOffset`)) (`self.DeltaSeconds`) (`self.InterpSpeed`)))
  (bind _rotationoffset (`self.CalculateRotationOffset` (`self.LeftFootRotation`) (`self.LeftFootFloorNormal`)))
  (set `self.LeftFootRotation` _rotationoffset)
  (bind _rotationoffset_2 (`self.CalculateRotationOffset` (`self.RightFootRotation`) (`self.RightFootFloorNormal`)))
  (set `self.RightFootRotation` _rotationoffset_2))

(fn `CalculateRotationOffset`
  (params (CurrentRotation :type "Rotator Structure") (FloorNormal :type "Vector Structure"))
  (returns (RotationOffset :type "Rotator Structure"))
  (bind _returnvalue (`Actor.GetActorUpVector` (`self.CharacterRef`)))
  (return (`KismetMathLibrary.RInterpTo` CurrentRotation (`KismetMathLibrary.RotatorFromAxisAndAngle` (`KismetMathLibrary.Cross_VectorVector` _returnvalue) (`KismetMathLibrary.DegAcos` (`KismetMathLibrary.Dot_VectorVector` _returnvalue FloorNormal))) (`self.DeltaSeconds`) (`self.InterpSpeed`))))

(fn `TraceFromRoot`
  (params (BoneName :type Name) (TraceDistBelowCapsule :type "Float (double-precision)"))
  (returns (ReturnValue :type "Float (double-precision)") (ImpactNormal :type "Vector Structure"))
  (locals (L_TraceDistBelowCapsule :type "Float (double-precision)") (L_BoneLocation :type "Vector Structure") (L_TraceStartLocation :type "Vector Structure") (L_TraceEndLocation :type "Vector Structure"))
  (bind (_l_bonelocation_x _l_bonelocation_y) (`KismetMathLibrary.BreakVector` (`local.L_BoneLocation`)))
  (bind (_l_bonelocation_x_2 _l_bonelocation_y_2) (`KismetMathLibrary.BreakVector` (`local.L_BoneLocation`)))
  (bind (_returnvalue_x _returnvalue_y _returnvalue_z) (`KismetMathLibrary.BreakVector` (`Actor.K2_GetActorLocation` (`self.CharacterRef`))))
  (bind (_returnvalue_x_2 _returnvalue_y_2 _returnvalue_z_2) (`KismetMathLibrary.BreakVector` (`Actor.K2_GetActorLocation` (`self.CharacterRef`))))
  (set `local.L_TraceDistBelowCapsule` TraceDistBelowCapsule)
  (set `local.L_BoneLocation` (`SceneComponent.GetSocketLocation` (`Character.Mesh` (`self.CharacterRef`)) BoneName))
  (set `local.L_TraceStartLocation` (`KismetMathLibrary.MakeVector` _l_bonelocation_x_2 _l_bonelocation_y_2 _returnvalue_z))
  (set `local.L_TraceEndLocation` (`KismetMathLibrary.MakeVector` _l_bonelocation_x _l_bonelocation_y (- _returnvalue_z_2 (+ (`CapsuleComponent.GetScaledCapsuleHalfHeight` (`Character.CapsuleComponent` (`self.CharacterRef`))) (`local.L_TraceDistBelowCapsule`)))))
  (bind (_outhit _returnvalue) (`KismetSystemLibrary.LineTraceSingle` (`local.L_TraceStartLocation`) (`local.L_TraceEndLocation`) "TraceTypeQuery2" true))
  (bind (_bblockinghit _binitialoverlap _time _distance _location _impactpoint _normal _impactnormal) (`GameplayStatics.BreakHitResult` _outhit))
  (return (`KismetMathLibrary.SelectFloat` (- (`KismetMathLibrary.VSize` (- (`local.L_TraceStartLocation`) _location)) (`CapsuleComponent.GetScaledCapsuleHalfHeight` (`Character.CapsuleComponent` (`self.CharacterRef`)))) 0.0 _returnvalue) _impactnormal))