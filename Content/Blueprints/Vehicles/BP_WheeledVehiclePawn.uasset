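; BP_WheeledVehiclePawn is a drivable vehicle pawn that the player character can approach and exit.
; Its trigger box sets NearCar and CarRef on an overlapping BP_Character, clears NearCar when it leaves, and prints French debug messages.
; Pressing Interact moves the stored character to SpawnLocation keeping only its yaw, restores visibility and collision, and has player controller 0 possess it again.
; Entering the vehicle is not handled in this graph.
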(event `self.TriggerBox.OnComponentBeginOverlap`
  (params (OverlappedComponent :type "PrimitiveComponent Object Reference") (OtherActor :type "Actor Object Reference") (OtherComp :type "PrimitiveComponent Object Reference") (OtherBodyIndex :type Integer) (bFromSweep :type Boolean) (SweepResult :type "HitResult Structure (by ref)"))
  ;[1 1 1] Detect Player
  (bind _asbp_character (cast `/Game/Blueprints/BP_Character` OtherActor))
  (set `/Game/Blueprints/BP_Character.NearCar` true _asbp_character)
  (set `/Game/Blueprints/BP_Character.CarRef` self _asbp_character)
  (`KismetSystemLibrary.PrintString` "BP_WheeledVehiclePawn --> Appuie sur E" true true (struct :`R` 1.0 :`G` 0.566909 :`A` 1.0) 5.0))

(event `self.TriggerBox.OnComponentEndOverlap`
  (params (OverlappedComponent :type "PrimitiveComponent Object Reference") (OtherActor :type "Actor Object Reference") (OtherComp :type "PrimitiveComponent Object Reference") (OtherBodyIndex :type Integer))
  ;[1 1 1] Detect Player
  (bind _asbp_character (cast `/Game/Blueprints/BP_Character` OtherActor))
  (set `/Game/Blueprints/BP_Character.NearCar` false _asbp_character)
  (`KismetSystemLibrary.PrintString` "BP_WheeledVehiclePawn --> la t'es loin" true true (struct :`R` 1.0 :`G` 0.456733 :`B` 0.496561 :`A` 1.0) 5.0))

(event `InputAction|Interact`
  (params (Key :type "Key Structure"))
  (bind _characterref (`self.CharacterRef`))
  (bind (_returnvalue_location _returnvalue_rotation) (`KismetMathLibrary.BreakTransform` (`SceneComponent.K2_GetComponentToWorld` (`self.SpawnLocation`))))
  ;[1 1 1] Sortir du véhicule
  (:`Pressed`
    (`self.K2_SetActorTransform` _characterref (`KismetMathLibrary.MakeTransform` _returnvalue_location (`KismetMathLibrary.MakeRotator` 0.0 0.0 (.yaw _returnvalue_rotation))) false false)
    (`self.SetActorHiddenInGame` _characterref false)
    (`self.SetActorEnableCollision` _characterref true)
    (`Controller.Possess` (`GameplayStatics.GetPlayerController` 0) _characterref)))

(fn `UserConstructionScript`)