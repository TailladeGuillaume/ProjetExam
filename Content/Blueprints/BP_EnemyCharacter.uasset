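; BP_EnemyCharacter is an enemy character Blueprint that distinguishes weak spot hits from base hits when it receives point damage.
; It switches on the hit physical material's surface type, scaling damage by a multiplier for weak spots and treating all other surfaces as base spots.
; The results are only printed as colored debug messages; no health is changed.
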(event `self.ReceivePointDamage`
  (params (Damage :type "Float (single-precision)") (DamageType :type "DamageType Object Reference") (HitLocation :type "Vector Structure") (HitNormal :type "Vector Structure") (HitComponent :type "PrimitiveComponent Object Reference") (BoneName :type Name) (ShotFromDirection :type "Vector Structure") (InstigatedBy :type "Controller Object Reference") (DamageCauser :type "Actor Object Reference") (HitInfo :type "HitResult Structure (by ref)"))
  (`KismetSystemLibrary.PrintString` "BP_EnemyCharacter --> Event Point Damage" true true (struct :`R` 1.0 :`B` 0.829997 :`A` 1.0))
  (switch `EPhysicalSurface` (`PhysicalMaterial.SurfaceType` (`.PhysMat` (`GameplayStatics.BreakHitResult` HitInfo)))
    (:`SurfaceType_Default`
      (`KismetSystemLibrary.PrintString` (`KismetStringLibrary.Concat_StrStr` "BP_EnemyCharacter --> BaseSpot : " (`KismetStringLibrary.Conv_DoubleToString` Damage)) true true (struct :`R` 1.0 :`G` 0.929221 :`B` 0.208059 :`A` 1.0) :!label _label))
    (:`SurfaceType1`
      (`KismetSystemLibrary.PrintString` (`KismetStringLibrary.Concat_StrStr` "BP_EnemyCharacter --> WeakSpot : " (`KismetStringLibrary.Conv_DoubleToString` (* Damage (`self.WeakSpot_DamageMultiplier`)))) true true (struct :`R` 1.0 :`G` 0.038955 :`A` 1.0)))
    (:`SurfaceType2`
      (goto _label))))

(fn `UserConstructionScript`)