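; BP_Character_Player is the player character Blueprint that sets up its on-screen UI and adjusts the camera to the player's state.
; On BeginPlay it creates the player HUD and crosshair widgets, then refreshes the life and stamina bars.
; Each Tick it switches the spring arm on EPlayerState between a close shoulder-offset Combat view and a farther centered Travel view, then prints walk-speed debug text.
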(event `self.ReceiveBeginPlay`
  (`parent.ReceiveBeginPlay`)
  ;[1 0.3471 0.9571] Set Widget Player
  (bind _returnvalue (`|CreateWidget` "/Game/Widgets/Widget_Player.Widget_Player_C" (`GameplayStatics.GetPlayerController` 0)))
  (`UserWidget.AddToViewport` _returnvalue 0)
  (set `self.WidgetPlayerRef` _returnvalue)
  ;[0.6325 1 0.5487] Update Bar
  (`/Game/Widgets/Widget_Player.UpdateProgressBarLife` (`self.WidgetPlayerRef`))
  (`/Game/Widgets/Widget_Player.UpdateProgressBarStamina` (`self.WidgetPlayerRef`))
  ;[1 0.1962 0.246] Set Widget CrossHair
  (bind _returnvalue_2 (`|CreateWidget` "/Game/Widgets/Widget_CrossHair.Widget_CrossHair_C" (`GameplayStatics.GetPlayerController` 0)))
  (`UserWidget.AddToViewport` _returnvalue_2 0)
  (set `self.WidgetCrossHairRef` _returnvalue_2))

(event `self.ReceiveTick`
  (params (DeltaSeconds :type "Float (single-precision)"))
  (bind _springarm (`self.SpringArm`))
  (`parent.ReceiveTick` DeltaSeconds)
  (`|ExecutionSequence`
    (:`then_0`
      ;[1 1 1] Manage Spring Arm
      (switch `/Game/Blueprints/EPlayerState` (`self.EPlayerState`)
        (:`NewEnumerator0`
          (set `SpringArmComponent.TargetArmLength` 200.0 _springarm)
          (set `SpringArmComponent.SocketOffset` (0.0 50.0 -10.0) _springarm))
        (:`NewEnumerator1`
          (set `SpringArmComponent.TargetArmLength` 400.0 _springarm)
          (set `SpringArmComponent.SocketOffset` (0.0 0.0 0.0) _springarm))))
    (:`then_1`
      ;[0 1 0.0352] Debug
      (`KismetSystemLibrary.PrintString` (`KismetStringLibrary.Concat_StrStr` "BP_Character_Player / TravelSpeed : " (`KismetStringLibrary.Conv_DoubleToString` (`self.TravelWalkSpeed`)) " / CombatSpeed : " (`KismetStringLibrary.Conv_DoubleToString` (`self.CombatWalkSpeed`)) " / MaxWalkSpeed : " (`KismetStringLibrary.Conv_DoubleToString` (`CharacterMovementComponent.MaxWalkSpeed` (`self.CharacterMovement`)))) true true (struct :`G` 1.0 :`B` 0.061501 :`A` 1.0) 0.0))))

(fn `UserConstructionScript`
  (`parent.UserConstructionScript`))