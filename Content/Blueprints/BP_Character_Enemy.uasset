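; Enemy character that wanders the level, takes point damage with weak spots and shows a life bar widget.
; Point damage reads the hit physical surface, multiplies Weak Spot hits, calls LooseLife, then refreshes the bar, with debug prints throughout.
; Tick drives wandering through delayed AIMoveTo calls to random reachable points, and stops then destroys the actor once IsDead.
; A move-to-player chase block exists but is never run.
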(event `self.ReceiveBeginPlay`
  (`parent.ReceiveBeginPlay`)
  ;[0.6325 1 0.5487] Update Bar
  (bind _aswidget_enemy_life (cast `/Game/Widgets/Widget_EnemyLife` (`WidgetComponent.GetUserWidgetObject` (`self.WidgetLifeBar`))))
  (bind _output_get (set `self.WidgetRef` _aswidget_enemy_life))
  (`/Game/Widgets/Widget_EnemyLife.UpdateEnemyBar` _output_get self))

(event `self.ReceivePointDamage`
  (params (Damage :type "Float (single-precision)") (DamageType :type "DamageType Object Reference") (HitLocation :type "Vector Structure") (HitNormal :type "Vector Structure") (HitComponent :type "PrimitiveComponent Object Reference") (BoneName :type Name) (ShotFromDirection :type "Vector Structure") (InstigatedBy :type "Controller Object Reference") (DamageCauser :type "Actor Object Reference") (HitInfo :type "HitResult Structure (by ref)"))
  (bind _returnvalue (* (`self.PointDamage_TakenDamage`) (`self.WeakSpot_DamageMultiplier`)))
  ;[1 1 1] Event Point Damage
  (set `self.PointDamage_TakenDamage` Damage)
  (`KismetSystemLibrary.PrintString` "BP_Character_Enemy --> Event Point Damage" true true (struct :`R` 1.0 :`B` 0.829997 :`A` 1.0))
  (switch `EPhysicalSurface` (`PhysicalMaterial.SurfaceType` (`.PhysMat` (`GameplayStatics.BreakHitResult` HitInfo)))
    (:`SurfaceType_Default`
      (`KismetSystemLibrary.PrintString` (`KismetStringLibrary.Concat_StrStr` "BP_Character_Enemy --> BaseSpot : " (`KismetStringLibrary.Conv_DoubleToString` (`self.PointDamage_TakenDamage`))) true true (struct :`R` 1.0 :`G` 0.929221 :`B` 0.208059 :`A` 1.0) :!label _label)
      (`self.LooseLife` (`self.PointDamage_TakenDamage`)))
    (:`SurfaceType1`
      (`KismetSystemLibrary.PrintString` (`KismetStringLibrary.Concat_StrStr` "BP_Character_Enemy --> WeakSpot : " (`KismetStringLibrary.Conv_DoubleToString` _returnvalue)) true true (struct :`R` 1.0 :`G` 0.038955 :`A` 1.0))
      (`self.LooseLife` _returnvalue))
    (:`SurfaceType2`
      (goto _label)))
  (`KismetSystemLibrary.PrintString` (`KismetStringLibrary.Concat_StrStr` "BP_Character_Enemy --> UpdateProgressBarLife / CurrentLife : " (`KismetStringLibrary.Conv_DoubleToString` (`self.CurrentLife`)) " / MaxLife : " (`KismetStringLibrary.Conv_DoubleToString` (`self.MaxLife`))) true true (struct :`R` 1.0 :`G` 0.826078 :`B` 0.107261 :`A` 1.0) 5.0)
  ;[0.9772 0.2917 1] Update Life Bar
  (bind _widgetref (`self.WidgetRef`)
    (:`then`
      (`/Game/Widgets/Widget_EnemyLife.UpdateEnemyBar` _widgetref self))
    (:`else`)))

(event `self.ReceiveTick`
  (params (DeltaSeconds :type "Float (single-precision)"))
  (`parent.ReceiveTick` DeltaSeconds)
  ;[0.3511 0.7975 1] Verif
  (if (`self.IsDead`)
    (`Controller.StopMovement` (`AIBlueprintHelperLibrary.GetAIController` self))
    (`KismetSystemLibrary.Delay` 1.0)
    (`self.K2_DestroyActor`)
    (elif (not (`self.AI_IsMoving`))
      (`KismetSystemLibrary.Delay` 2.0)
      (set `self.AI_IsMoving` true)
      (`|AIMoveTo` self (`NavigationSystemV1.K2_GetRandomReachablePointInRadius` (`self.K2_GetActorLocation`) 2000.0 null null) null
        (:`OnSuccess`
          _)
        (:`OnFail`
          _))
      (set `self.AI_IsMoving` false))))

(fn `UserConstructionScript`
  (`parent.UserConstructionScript`))